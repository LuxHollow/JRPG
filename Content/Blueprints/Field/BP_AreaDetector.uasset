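; BP_AreaDetector is a field trigger that tells the game mode which area the player enters when leaving its box.
; When a BP_FieldPlayer ends overlap, it takes the dot product of ArrowRed's forward vector and the direction from the arrow to the player.
; A non-negative result sends AreaRed through IChangeAreaMessage; a negative one sends AreaBlue, so the exit side decides the area.
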(event `self.Box.OnComponentEndOverlap`
  (params (OverlappedComponent :type "PrimitiveComponent Object Reference") (OtherActor :type "Actor Object Reference") (OtherComp :type "PrimitiveComponent Object Reference") (OtherBodyIndex :type Integer))
  (bind _arrowred (`self.ArrowRed`))
  (`KismetSystemLibrary.IsObjectOfSoftClass` OtherActor "/Game/Blueprints/Field/BP_FieldPlayer.BP_FieldPlayer_C"
    (:`True`
      (if (>= (`KismetMathLibrary.Dot_VectorVector` (`SceneComponent.GetForwardVector` _arrowred) (`KismetMathLibrary.GetForwardVector` (`KismetMathLibrary.FindLookAtRotation` (`SceneComponent.K2_GetComponentLocation` _arrowred) (`self.K2_GetActorLocation` OtherActor)))) 0.0)
        (message `/Game/Definitions/Interfaces/BPI_AreaControl.I_ChangeArea` (`GameplayStatics.GetGameMode`) (`self.AreaRed`))
        (else
          (message `/Game/Definitions/Interfaces/BPI_AreaControl.I_ChangeArea` (`GameplayStatics.GetGameMode`) (`self.AreaBlue`)))))))

(fn `UserConstructionScript`)