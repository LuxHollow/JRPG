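; Player-controlled party leader for field exploration, with movement, pause, interaction and random battle encounters.
; On BeginPlay it applies the first living member's data to itself and spawns followers for the rest.
; Distance accumulated while moving triggers encounters at randomized thresholds, storing position and playing a transition before entering battle if the area has a battle map.
; Interaction sphere-traces forward and uses the first interactable hit.
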(event `self.ReceiveBeginPlay`
  (`parent.ReceiveBeginPlay`)
  (message `/Game/Definitions/Interfaces/BPI_UIControl.I_InitWidgetField` (`GameplayStatics.GetPlayerController` 0))
  (bind _widgetfield (message `/Game/Definitions/Interfaces/BPI_UIControl.I_GetWidgetField` (`GameplayStatics.GetPlayerController` 0)))
  (`/Game/UI/Widgets/WBP_Transition.PlayOpenAnim` (`/Game/UI/Widgets/WBP_Field.WBP_Transition` _widgetfield))
  (`self.InitializeParty`)
  (`self.DecideEncounterDistance`))

(event `self.ReceivePossessed`
  (params (NewController :type "Controller Object Reference"))
  (`parent.ReceivePossessed` NewController)
  (bind _asplayer_controller (cast `PlayerController` (`self.GetController`)))
  (`EnhancedInputSubsystemInterface.AddMappingContext` (pcsubsystem `EnhancedInputLocalPlayerSubsystem` _asplayer_controller) "/Game/Inputs/Field/IMC_Field.IMC_Field" 0 (struct)))

(event `EnhancedInput|/Game/Inputs/Field/Actions/IA_Move`
  (params (ActionValue :type "Vector2D Structure") (ElapsedSeconds :type "Float (double-precision)") (TriggeredSeconds :type "Float (double-precision)") (InputAction :type "InputAction Object Reference" :default "/Game/Inputs/Field/Actions/IA_Move.IA_Move"))
  (bind (_x _y) (`KismetMathLibrary.BreakVector2D` ActionValue))
  (:`Triggered`
    (`self.AddMovementInput` (1.0 0.0 0.0) _x)
    (`self.AddMovementInput` (0.0 1.0 0.0) _y)
    (set `self.DistanceSinceEncounter` (+ (`self.DistanceSinceEncounter`) (* (`KismetMathLibrary.VSize` (`self.GetVelocity`)) (`GameplayStatics.GetWorldDeltaSeconds`))))
    (if (>= (`self.DistanceSinceEncounter`) (`self.EncounterDistance`))
      (`self.StartEncounter`)
      (`self.ResetDistance`))))

(event `EnhancedInput|/Game/Inputs/Field/Actions/IA_Interect`
  (params (ActionValue :type Boolean) (ElapsedSeconds :type "Float (double-precision)") (TriggeredSeconds :type "Float (double-precision)") (InputAction :type "InputAction Object Reference" :default "/Game/Inputs/Field/Actions/IA_Interect.IA_Interect"))
  (:`Started`
    (`self.TryInteract`)))

(event `EnhancedInput|/Game/Inputs/Field/Actions/IA_Pause`
  (params (ActionValue :type Boolean) (ElapsedSeconds :type "Float (double-precision)") (TriggeredSeconds :type "Float (double-precision)") (InputAction :type "InputAction Object Reference" :default "/Game/Inputs/Field/Actions/IA_Pause.IA_Pause"))
  (:`Started`
    (message `/Game/Definitions/Interfaces/BPI_Pausable.I_SetGameStatePaused` (`GameplayStatics.GetGameMode`) true)))

(event `StartEncounter`
  (bind _areadata (message `/Game/Definitions/Interfaces/BPI_AreaControl.I_GetCurrentAreaData` (`GameplayStatics.GetGameMode`)))
  (bind _battlemap_worldasset (break `SoftWorldReference` (`/Game/Data/DataAssets/AreaData/PDA_AreaData.BattleMap` _areadata)))
  (if (`KismetSystemLibrary.IsValidSoftObjectReference` _battlemap_worldasset)
    (`self.StoreFieldPositionOnInstance`)
    (bind _widgetfield (message `/Game/Definitions/Interfaces/BPI_UIControl.I_GetWidgetField` (`GameplayStatics.GetPlayerController` 0)))
    (`/Game/UI/Widgets/WBP_Transition.PlayCloseAnim` (`/Game/UI/Widgets/WBP_Field.WBP_Transition` _widgetfield))
    (message `/Game/Definitions/Interfaces/BPI_UIControl.I_DisableFieldInputs` (`GameplayStatics.GetPlayerController` 0))
    (`KismetSystemLibrary.RetriggerableDelay` (`/Game/Data/DataAssets/GlobalVariables/PDA_GlobalVariables.TransitionDelay` (`/Game/Definitions/FunctionLibraries/BPFL_CORE.GetGlobalVariables`)))
    (message `/Game/Definitions/Interfaces/BPI_AreaControl.I_EnterBattleArea` (`GameplayStatics.GetGameMode`))))

(fn `DecideEncounterDistance`
  (bind (_encounterdistance_x _encounterdistance_y) (`KismetMathLibrary.BreakVector2D` (`/Game/Data/DataAssets/GlobalVariables/PDA_GlobalVariables.EncounterDistance` (`/Game/Definitions/FunctionLibraries/BPFL_CORE.GetGlobalVariables`))))
  (set `self.EncounterDistance` (`KismetMathLibrary.RandomFloatInRange` _encounterdistance_x _encounterdistance_y)))

(fn `InitializeParty`
  (locals (PartyMembers :type "Array of /Game/Data/DataAssets/PartyMemberData/PDA_PartyMemberData Object Reference"))
  (bind _alivemembers (message `/Game/Definitions/Interfaces/BPI_InstanceStorage.I_GetAlivePartyMembers` (`GameplayStatics.GetGameInstance`)))
  (set `local.PartyMembers` _alivemembers)
  (`self.ApplyMemberData` (`|GetArrayItem` (`local.PartyMembers`)))
  (`KismetArrayLibrary.Array_Remove` (`local.PartyMembers`)) ; Ignore Leader
  (for (_array_element _array_index) (`local.PartyMembers`)
    (bind _returnvalue (`|SpawnActorFromClass` "/Game/Blueprints/Field/BP_FieldFollower.BP_FieldFollower_C" (`self.GetTransform`) "AlwaysSpawn" "MultiplyWithRoot" null null))
    (`self.ApplyMemberData` _returnvalue _array_element (+ _array_index 1))
    (set `/Game/Blueprints/Field/BP_FieldFollower.FollowTarget` self _returnvalue)))

(fn `ResetDistance`
  (set `self.DistanceSinceEncounter` 0.0)
  (`self.DecideEncounterDistance`))

(fn `StoreFieldPositionOnInstance`
  (message `/Game/Definitions/Interfaces/BPI_InstanceStorage.I_StoreFieldPosition` (`GameplayStatics.GetGameInstance`) (`self.GetTransform`)))

(fn `TryInteract`
  (bind _returnvalue (`self.K2_GetActorLocation`))
  (bind _outhits (`KismetSystemLibrary.SphereTraceMultiForObjects` :`Start` _returnvalue :`End` (+ _returnvalue (* (`self.GetActorForwardVector`) (`self.InteractDistance`))) :`Radius` (`self.InteractRadius`) :`ObjectTypes` (`|MakeArray` "ObjectTypeQuery2" "ObjectTypeQuery3" :!type "EObjectTypeQuery Enum") :`DrawDebugType` "ForDuration"))
  (for _array_element _outhits
    (bind (_bblockinghit _binitialoverlap _time _distance _location _impactpoint _normal _impactnormal _physmat _hitactor) (`GameplayStatics.BreakHitResult` _array_element))
    (bind _caninteract (message `/Game/Definitions/Interfaces/BPI_Interactable.I_CanInteract` _hitactor))
    (if _caninteract
      (message `/Game/Definitions/Interfaces/BPI_Interactable.I_Interact` _hitactor)
      (break))))

(fn `UserConstructionScript`
  (`parent.UserConstructionScript`))