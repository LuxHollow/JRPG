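; AC_Shaker is a component that gives a scene component, supplied through Initialize, a timed side-to-side shake along its relative X axis.
; StartShake runs a looping timer and waits on a retriggerable delay before calling EndShake.
; ShakeOnce uses a FlipFlop to alternate X between small positive and negative offsets.
; EndShake clears the stored timer and resets relative X to zero rather than its original value.
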(event `self.ReceiveBeginPlay`)

(event `StartShake`
  (bind _returnvalue (`KismetSystemLibrary.K2_SetTimerDelegate` (`|CreateDelegate` :!event `ShakeOnce`) (`self.ShakeInterval`) true))
  (set `self.ShakeHandle` _returnvalue)
  (`KismetSystemLibrary.RetriggerableDelay` (`self.ShakeDuration`))
  (`self.EndShake`))

(event `ShakeOnce`
  (bind (_relativelocation_x _relativelocation_y _relativelocation_z) (`KismetMathLibrary.BreakVector` (`SceneComponent.RelativeLocation` (`self.CompToShake`))))
  (bind _isa (`/Engine/EditorBlueprintResources/StandardMacros.FlipFlop`)
    (:`A`
      _)
    (:`B`
      _))
  (`SceneComponent.K2_SetRelativeLocation` (`self.CompToShake`) (`KismetMathLibrary.MakeVector` (`KismetMathLibrary.SelectFloat` 5.0 -5.0 _isa) _relativelocation_y _relativelocation_z) false false))

(event `EndShake`
  (bind (_relativelocation_x _relativelocation_y _relativelocation_z) (`KismetMathLibrary.BreakVector` (`SceneComponent.RelativeLocation` (`self.CompToShake`))))
  (`KismetSystemLibrary.K2_ClearAndInvalidateTimerHandle` (`self.ShakeHandle`))
  (`SceneComponent.K2_SetRelativeLocation` (`self.CompToShake`) (`KismetMathLibrary.MakeVector` 0.0 _relativelocation_y _relativelocation_z) false false))

(fn `Initialize`
  (params (CompToShake :type "SceneComponent Object Reference"))
  (set `self.CompToShake` CompToShake))