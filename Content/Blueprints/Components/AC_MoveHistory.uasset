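; Actor component that records a trail of its owner's recent transforms and serves delayed positions by member ID, apparently for followers in a line.
; A looping timer samples the owner and stores a transform only when it has moved over one unit, dropping the oldest beyond a maximum count.
; GetEntryForMemberIndex steps back from the newest entry by member ID times a fixed spacing, flagging whether that entry exists.
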(event `self.ReceiveBeginPlay`
  (`KismetSystemLibrary.K2_SetTimerDelegate` (delegate `TimeStep`) (`self.UpdateInterval`) true true))

(event `TimeStep`
  (`self.AddTransform` (`Actor.GetTransform` (`self.GetOwner`))))

(fn `AddTransform`
  (params (TransformToAdd :type "Transform Structure"))
  (bind _transformtoadd_location (`KismetMathLibrary.BreakTransform` (`local.TransformToAdd`)))
  (bind _lasttransform_location (`KismetMathLibrary.BreakTransform` (`self.LastTransform`)))
  (if (> (`KismetMathLibrary.Vector_Distance` _lasttransform_location _transformtoadd_location) 1.0)
    (set `self.LastTransform` (`local.TransformToAdd`))
    (`KismetArrayLibrary.Array_Add` (`self.PastTransform`) (`local.TransformToAdd`))
    (if (> (`KismetArrayLibrary.Array_Length` (`self.PastTransform`)) (`self.MaxEntries`))
      (`KismetArrayLibrary.Array_Remove` (`self.PastTransform`)))))

(fn `GetEntryForMemberIndex`
  (params (MemberID :type Integer))
  (returns (TargetTransform :type "Transform Structure (by ref)") (IsValid :type Boolean))
  (locals (CheckEntry :type Integer))
  (set `local.CheckEntry` (- (`KismetArrayLibrary.Array_LastIndex` (`self.PastTransform`)) (* MemberID (`self.EntrySteps`))))
  (if (`KismetArrayLibrary.Array_IsValidIndex` (`self.PastTransform`) (`local.CheckEntry`))
    (return (`|GetArrayItem` (`self.PastTransform`) (`local.CheckEntry`)) true)
    (else
      (return (struct) false))))