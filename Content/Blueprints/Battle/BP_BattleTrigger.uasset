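; BP_BattleTrigger is a box trigger that sends the field player into a battle.
; On overlap with BP_FieldPlayer, it continues only if the game mode's current area data has a valid battle map soft reference.
; It then stores the field position on the instance, plays the transition close animation, disables field inputs and, after the global transition delay, tells the game mode to enter the battle area through interface messages.
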(event `self.Box.OnComponentBeginOverlap`
  (params (OverlappedComponent :type "PrimitiveComponent Object Reference") (OtherActor :type "Actor Object Reference") (OtherComp :type "PrimitiveComponent Object Reference") (OtherBodyIndex :type Integer) (bFromSweep :type Boolean) (SweepResult :type "HitResult Structure (by ref)"))
  (bind _asbp_field_player (cast `/Game/Blueprints/Field/BP_FieldPlayer` OtherActor))
  (bind _areadata (message `/Game/Definitions/Interfaces/BPI_AreaControl.I_GetCurrentAreaData` (`GameplayStatics.GetGameMode`)))
  (bind _battlemap_worldasset (break `SoftWorldReference` (`/Game/Data/DataAssets/AreaData/PDA_AreaData.BattleMap` _areadata)))
  (if (`KismetSystemLibrary.IsValidSoftObjectReference` _battlemap_worldasset)
    (`/Game/Blueprints/Field/BP_FieldPlayer.StoreFieldPositionOnInstance` _asbp_field_player)
    (bind _widgetfield (message `/Game/Definitions/Interfaces/BPI_UIControl.I_GetWidgetField` (`GameplayStatics.GetPlayerController` 0)))
    (`/Game/UI/Widgets/WBP_Transition.PlayCloseAnim` (`/Game/UI/Widgets/WBP_Field.WBP_Transition` _widgetfield))
    (message `/Game/Definitions/Interfaces/BPI_UIControl.I_DisableFieldInputs` (`GameplayStatics.GetPlayerController` 0))
    (`KismetSystemLibrary.RetriggerableDelay` (`/Game/Data/DataAssets/GlobalVariables/PDA_GlobalVariables.TransitionDelay` (`/Game/Definitions/FunctionLibraries/BPFL_CORE.GetGlobalVariables`)))
    (message `/Game/Definitions/Interfaces/BPI_AreaControl.I_EnterBattleArea` (`GameplayStatics.GetGameMode`))))

(fn `UserConstructionScript`)