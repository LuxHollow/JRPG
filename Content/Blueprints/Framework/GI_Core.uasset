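; Game Instance for a party-based RPG, holding party members and their states, inventory, triggered IDs and field position across levels.
; On Init it seeds each member's HP, MP and level from initial data and creates the save object.
; Interface calls read and update this data, with stack-capped items and knocked-out filtering for alive members.
; SaveGameData copies it, plus the pawn's current transform, level and area, into a single slot.
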(event `self.ReceiveInit`
  (for _array_element (`self.PartyMembers`)
    (bind (_maxhp _maxmp) (break `/Game/Definitions/Structs/S_CharAttributes` (`/Game/Data/DataAssets/BattleCharData/PDA_BattleCharData.InitialAttributes` (`/Game/Data/DataAssets/PartyMemberData/PDA_PartyMemberData.BattleCharData` _array_element))))
    (`KismetArrayLibrary.Array_Add` (`self.PartyStates`) (make `/Game/Definitions/Structs/S_CharState` _maxhp _maxmp 1)))
  (bind _returnvalue (`GameplayStatics.CreateSaveGameObject` "/Game/Blueprints/SaveLoad/BP_SaveGame.BP_SaveGame_C"))
  (set `self.SaveGame` _returnvalue))

(event `/Game/Definitions/Interfaces/BPI_InstanceStorage.I_StoreFieldPosition`
  (params (LastFieldTransform :type "Transform Structure"))
  (`self.StoreFieldPosition` LastFieldTransform))

(event `/Game/Definitions/Interfaces/BPI_InstanceStorage.I_StorePartyStates`
  (params (partyMembers :type "Array of /Game/Blueprints/Battle/BattleChars/BP_BattleChar_BASE Object Reference (by ref)"))
  (`self.StorePartyStates` partyMembers))

(event `/Game/Definitions/Interfaces/BPI_InstanceStorage.I_AddItemToInventory`
  (params (ItemData :type "/Game/Data/DataAssets/ItemData/PDA_ItemData Object Reference") (Amount :type Integer))
  (`self.AddItemToInventory` ItemData Amount))

(event `/Game/Definitions/Interfaces/BPI_InstanceStorage.I_AddTriggeredID`
  (params (ID :type Name))
  (`self.AddTriggeredID` ID))

(fn `AddItemToInventory`
  (params (ItemData :type "/Game/Data/DataAssets/ItemData/PDA_ItemData Object Reference") (Amount :type Integer))
  (locals (NewAmount :type Integer))
  (bind _output_get (set `local.NewAmount` (`KismetMathLibrary.Min` (+ (`BlueprintMapLibrary.Map_Find` (`self.Inventory`) (`local.ItemData`)) (`local.Amount`)) (`/Game/Data/DataAssets/ItemData/PDA_ItemData.MaxStackSize` (`local.ItemData`)))))
  (`BlueprintMapLibrary.Map_Add` (`self.Inventory`) (`local.ItemData`) _output_get))

(fn `AddTriggeredID`
  (params (ID :type "Name (by ref)"))
  (`BlueprintMapLibrary.Map_Add` (`self.TriggeredIDs`) ID true))

(fn `GetAlivePartyMembers`
  (returns (LiveMembers :type "Array of /Game/Data/DataAssets/PartyMemberData/PDA_PartyMemberData Object Reference"))
  (locals (Members :type "Array of /Game/Data/DataAssets/PartyMemberData/PDA_PartyMemberData Object Reference"))
  (for (_array_element _array_index) (`self.PartyStates`)
    (if (not (`.IsKnockedOut_15_3E80255F498CDBA2F61A9BB5BB5AF49D` (break `/Game/Definitions/Structs/S_CharState` _array_element)))
      (`KismetArrayLibrary.Array_Add` (`local.Members`) (`|GetArrayItem` (`self.PartyMembers`) _array_index))))
  (return (`local.Members`)))

(fn `I_GetAlivePartyMembers`
  (returns (AliveMembers :type "Array of /Game/Data/DataAssets/PartyMemberData/PDA_PartyMemberData Object Reference"))
  (bind _livemembers (`self.GetAlivePartyMembers`))
  (return _livemembers))

(fn `I_GetGlobalVariables`
  (returns (GlobalVariables :type "/Game/Data/DataAssets/GlobalVariables/PDA_GlobalVariables Object Reference"))
  (return (`self.GlobalVariables`)))

(fn `I_GetInventory`
  (returns (Inventory :type "Map of /Game/Data/DataAssets/ItemData/PDA_ItemData Object Reference to Integer"))
  (return (`self.Inventory`)))

(fn `I_GetPartyMembers`
  (returns (PartyMembers :type "Array of /Game/Data/DataAssets/PartyMemberData/PDA_PartyMemberData Object Reference"))
  (return (`self.PartyMembers`)))

(fn `I_GetPartyStates`
  (returns (States :type "Array of /Game/Definitions/Structs/S_CharState Structure"))
  (return (`self.PartyStates`)))

(fn `I_GetPlayerFieldPosition`
  (returns (PlayerFieldPosition :type "/Game/Definitions/Structs/S_FieldPosition Structure"))
  (return (`self.PlayerFieldPosition`)))

(fn `I_IsIDTriggered`
  (params (ID :type Name))
  (returns (Value :type Boolean))
  (bind _returnvalue (`self.IsIDTriggered` ID))
  (return _returnvalue))

(fn `I_UseItemFromInventory`
  (params (ItemData :type "/Game/Data/DataAssets/ItemData/PDA_ItemData Object Reference"))
  (returns (FinalAmount :type Integer))
  (bind _finalamount (`self.UseItemFromInventory` ItemData))
  (return _finalamount))

(fn `IsIDTriggered`
  (params (ID :type "Name (by ref)"))
  (returns (ReturnValue :type Boolean))
  (return (`.ReturnValue` (`BlueprintMapLibrary.Map_Find` (`self.TriggeredIDs`) ID))))

(fn `SaveGameData`
  (set `/Game/Blueprints/SaveLoad/BP_SaveGame.PartyMembers` (`self.PartyMembers`) (`self.SaveGame`))
  (set `/Game/Blueprints/SaveLoad/BP_SaveGame.Inventory` (`self.Inventory`) (`self.SaveGame`))
  (set `/Game/Blueprints/SaveLoad/BP_SaveGame.TriggeredIDs` (`self.TriggeredIDs`) (`self.SaveGame`))
  (set `/Game/Blueprints/SaveLoad/BP_SaveGame.PartyStates` (`self.PartyStates`) (`self.SaveGame`))
  (set `/Game/Blueprints/SaveLoad/BP_SaveGame.DateTime` (`KismetMathLibrary.Now`) (`self.SaveGame`))
  (bind _areadata (message `/Game/Definitions/Interfaces/BPI_AreaControl.I_GetCurrentAreaData` (`GameplayStatics.GetGameMode`)))
  (bind _returnvalue (`GameplayStatics.GetCurrentLevelName` true))
  (set `/Game/Blueprints/SaveLoad/BP_SaveGame.PlayerFieldPosition` (make `/Game/Definitions/Structs/S_FieldPosition` _returnvalue (`Actor.GetTransform` (`GameplayStatics.GetPlayerPawn` 0)) _areadata) (`self.SaveGame`))
  (`GameplayStatics.SaveGameToSlot` (`self.SaveGame`) "0"))

(fn `StoreFieldPosition`
  (params (LastFieldTransform :type "Transform Structure"))
  (setmembers `/Game/Definitions/Structs/S_FieldPosition` :`StructRef` (`self.PlayerFieldPosition`) :`LastFieldTransform` LastFieldTransform)
  (bind _areadata (message `/Game/Definitions/Interfaces/BPI_AreaControl.I_GetCurrentAreaData` (`GameplayStatics.GetGameMode`)))
  (bind _returnvalue (`GameplayStatics.GetCurrentLevelName` true))
  (setmembers `/Game/Definitions/Structs/S_FieldPosition` :`StructRef` (`self.PlayerFieldPosition`) :`FieldLevelName` _returnvalue :`AreaInfo` _areadata))

(fn `StorePartyStates`
  (params (PartyMembers :type "Array of /Game/Blueprints/Battle/BattleChars/BP_BattleChar_BASE Object Reference"))
  (for (_array_element _array_index) PartyMembers
    (`KismetArrayLibrary.Array_Set` (`self.PartyStates`) _array_index (`/Game/Blueprints/Components/AC_BattleStats.State` (`/Game/Blueprints/Battle/BattleChars/BP_BattleChar_BASE.AC_BattleStats` _array_element)) true)))

(fn `UseItemFromInventory`
  (params (ItemData :type "/Game/Data/DataAssets/ItemData/PDA_ItemData Object Reference"))
  (returns (FinalAmount :type Integer))
  (locals (NewAmount :type Integer))
  (set `local.NewAmount` (- (`BlueprintMapLibrary.Map_Find` (`self.Inventory`) (`local.ItemData`)) 1))
  (if (<= (`local.NewAmount`) 0)
    (`BlueprintMapLibrary.Map_Remove` (`self.Inventory`) (`local.ItemData`))
    (else
      (`BlueprintMapLibrary.Map_Add` (`self.Inventory`) (`local.ItemData`) (`local.NewAmount`))))
  (return (`local.NewAmount`)))