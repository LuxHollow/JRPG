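; Game mode for field exploration levels that spawns the player and tracks the current area, including its battle map.
; On BeginPlay it spawns and possesses BP_FieldPlayer at the field transform saved in the Game Instance, or at a PlayerStart when no field level is saved.
; Interface calls drive area changes, which fade in the new area name on the field widget, and battle entry, which opens the current area's battle level.
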(event `self.ReceiveBeginPlay`
  (`WidgetBlueprintLibrary.SetFocusToGameViewport`)
  (`self.SpawnPlayer`)
  (message `/Game/Definitions/Interfaces/BPI_UIControl.I_DeactivateUIControls` (`GameplayStatics.GetPlayerController` 0)))

(event `/Game/Definitions/Interfaces/BPI_AreaControl.I_ChangeArea`
  (params (NewArea :type "/Game/Data/DataAssets/AreaData/PDA_AreaData Object Reference"))
  (`self.ChangeArea` NewArea))

(event `/Game/Definitions/Interfaces/BPI_AreaControl.I_EnterBattleArea`
  (`self.EnterBattleArea`))

(fn `ChangeArea`
  (params (NewArea :type "/Game/Data/DataAssets/AreaData/PDA_AreaData Object Reference"))
  (if (`KismetTextLibrary.NotEqual_TextText` (`/Game/Data/DataAssets/AreaData/PDA_AreaData.AreaName` (`local.NewArea`)) (`/Game/Data/DataAssets/AreaData/PDA_AreaData.AreaName` (`self.CurrentAreaData`)))
    (set `self.CurrentAreaData` (`local.NewArea`))
    (bind _widgetfield (message `/Game/Definitions/Interfaces/BPI_UIControl.I_GetWidgetField` (`GameplayStatics.GetPlayerController` 0)))
    (`/Game/UI/Widgets/Field/WBP_AreaName.PlayFadeAnim` (`/Game/UI/Widgets/WBP_Field.WBP_AreaName` _widgetfield) (`/Game/Data/DataAssets/AreaData/PDA_AreaData.AreaName` (`self.CurrentAreaData`)))))

(fn `EnterBattleArea`
  (bind _battlemap_worldasset (break `SoftWorldReference` (`/Game/Data/DataAssets/AreaData/PDA_AreaData.BattleMap` (`self.CurrentAreaData`))))
  (`GameplayStatics.OpenLevelBySoftObjectPtr` _battlemap_worldasset))

(fn `I_GetCurrentAreaData`
  (returns (AreaData :type "/Game/Data/DataAssets/AreaData/PDA_AreaData Object Reference"))
  (return (`self.CurrentAreaData`)))

(fn `SpawnPlayer`
  (bind _playerfieldposition (message `/Game/Definitions/Interfaces/BPI_InstanceStorage.I_GetPlayerFieldPosition` (`GameplayStatics.GetGameInstance`)))
  (bind (_fieldlevelname _lastfieldtransform _areainfo) (break `/Game/Definitions/Structs/S_FieldPosition` _playerfieldposition))
  (set `self.CurrentAreaData` _areainfo)
  (if (`KismetStringLibrary.IsEmpty` _fieldlevelname)
    (bind _returnvalue (`GameplayStatics.GetActorOfClass` "/Script/Engine.PlayerStart"))
    (bind (_returnvalue_location _returnvalue_rotation) (`KismetMathLibrary.BreakTransform` (`self.GetTransform` _returnvalue)))
    (bind _returnvalue_2 (`|SpawnActorFromClass` "/Game/Blueprints/Field/BP_FieldPlayer.BP_FieldPlayer_C" (`KismetMathLibrary.MakeTransform` _returnvalue_location _returnvalue_rotation) "Undefined" "MultiplyWithRoot" null null))
    (`Controller.Possess` (`GameplayStatics.GetPlayerController` 0) _returnvalue_2)
    (else
      (bind _returnvalue_3 (`|SpawnActorFromClass` "/Game/Blueprints/Field/BP_FieldPlayer.BP_FieldPlayer_C" (`KismetMathLibrary.MakeTransform` (.location _lastfieldtransform) (.rotation _lastfieldtransform)) "Undefined" "MultiplyWithRoot" null null))
      (`Controller.Possess` (`GameplayStatics.GetPlayerController` 0) _returnvalue_3))))

(fn `UserConstructionScript`)